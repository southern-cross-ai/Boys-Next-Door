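; Combat game instance that loads and holds the hero data and team member save games.
; Load events read the HeroData and TeamMembers slots, cast each to its SaveGame class and cache it in a variable.
; Debug events overwrite those slots with newly created saves: hero data at class defaults and team members with a hardcoded UUID list.
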(event `Debug Set Hero Datas`
  (bind _returnvalue (`GameplayStatics.CreateSaveGameObject` "/Game/Combat/Blueprints/SaveGame/BP_CombatSaveGame_HeroData.BP_CombatSaveGame_HeroData_C"))
  (`GameplayStatics.SaveGameToSlot` _returnvalue "HeroData"))

(event `Debug Set Team Members`
  (bind _returnvalue (`GameplayStatics.CreateSaveGameObject` "/Game/Combat/Blueprints/SaveGame/BP_CombatSaveGame_TeamMembers.BP_CombatSaveGame_TeamMembers_C"))
  (set `/Game/Combat/Blueprints/SaveGame/BP_CombatSaveGame_TeamMembers.Team Member UUID List` (`|MakeArray` 5 8 7 6) _returnvalue)
  (`GameplayStatics.SaveGameToSlot` _returnvalue "TeamMembers"))

(event `Load Team Members`
  (bind _returnvalue (`GameplayStatics.LoadGameFromSlot` "TeamMembers"))
  (bind _asbp_combat_save_game_team_members (cast `/Game/Combat/Blueprints/SaveGame/BP_CombatSaveGame_TeamMembers` _returnvalue))
  (set `self.Team Members SaveGame` _asbp_combat_save_game_team_members))

(event `Load Hero Datas`
  (bind _returnvalue (`GameplayStatics.LoadGameFromSlot` "HeroData"))
  (bind _asbp_combat_save_game_hero_data (cast `/Game/Combat/Blueprints/SaveGame/BP_CombatSaveGame_HeroData` _returnvalue))
  (set `self.Hero Data SaveGame` _asbp_combat_save_game_hero_data))