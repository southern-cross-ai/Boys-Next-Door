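; Combat buff that lowers a target unit's physical or magical defense until the buff ends.
; Initialization reads type, percentage mode and modifier from the init data.
; Physical defense drops by percentage or flat amount, possibly below zero, while magical defense is set to zero, leaving modifier math unwired.
; ApplyBuff saves only physical Defense, which OnBuffEnded writes back to whichever stat was reduced, even magical.
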(event `self.ApplyBuff`
  (bind _bypercentage (`self.byPercentage`))
  (bind _returnvalue (`KismetSystemLibrary.GetObjectName` (`self.targetUnit`)))
  (`parent.ApplyBuff`)
  ;[1 1 1] reduce defense
  (set `self.initDefense` (`/Game/TurnBasedJRPGTemplate/Blueprints/Units/BP_UnitBase.defense` (`self.targetUnit`)))
  (if (`self.isPhysical`)
    (bind _newdefense (`self.Reduce Physical Defense` _bypercentage))
    (`KismetSystemLibrary.PrintString` (`KismetStringLibrary.Concat_StrStr` (`KismetStringLibrary.Concat_StrStr` (`KismetStringLibrary.Concat_StrStr` (`KismetStringLibrary.Concat_StrStr` _returnvalue "‘s phycisal defense has been reduced to ") (`KismetStringLibrary.Conv_IntToString` _newdefense)) ".  Was ") (`KismetStringLibrary.Conv_IntToString` (`self.initDefense`))))
    (else
      (bind _newdefense_2 (`self.Reduce Magical Defense` _bypercentage))
      (`KismetSystemLibrary.PrintString` (`KismetStringLibrary.Concat_StrStr` (`KismetStringLibrary.Concat_StrStr` (`KismetStringLibrary.Concat_StrStr` (`KismetStringLibrary.Concat_StrStr` _returnvalue "‘s magical defense has been reduced to ") (`KismetStringLibrary.Conv_IntToString` _newdefense_2)) ".  Was ") (`KismetStringLibrary.Conv_IntToString` (`self.initDefense`)))))))

(event `self.OnBuffEnded`
  (bind _targetunit (`self.targetUnit`))
  (bind _initdefense (`self.initDefense`))
  (`parent.OnBuffEnded`)
  ;[1 1 1] Restore defense
  (if (`self.isPhysical`)
    (set `/Game/TurnBasedJRPGTemplate/Blueprints/Units/BP_UnitBase.defense` _initdefense _targetunit)
    (else
      (set `/Game/TurnBasedJRPGTemplate/Blueprints/Units/BP_UnitBase.magicalDefense` _initdefense _targetunit)))
  (`KismetSystemLibrary.PrintString` (`KismetStringLibrary.Concat_StrStr` (`KismetStringLibrary.Concat_StrStr` (`KismetSystemLibrary.GetObjectName` (`self.targetUnit`)) "'s defense has been restored to ") (`KismetStringLibrary.Conv_IntToString` _initdefense))))

(fn `Initialization`
  (params (buffInitData :type "/Game/Combat/Blueprints/Skills/Buffs/BuffInitData Structure"))
  (bind (_isphysical _bypercentage _turnduration _modifierdamage) (break `/Game/Combat/Blueprints/Skills/Buffs/BuffInitData` buffInitData))
  (`parent.Initialization` buffInitData)
  (set `self.isPhysical` _isphysical)
  (set `self.byPercentage` _bypercentage)
  (set `self.defenseModifier` _modifierdamage))

(fn `Reduce Magical Defense`
  (params (isPercentage :type Boolean))
  (returns (newDefense :type Integer))
  (if isPercentage
    ;[1 1 1] Reduce defense by percentage
    (bind _output_get (set `/Game/TurnBasedJRPGTemplate/Blueprints/Units/BP_UnitBase.magicalDefense` 0 (`self.targetUnit`)))
    (return _output_get)
    (else
      ;[1 1 1] Reduce defense by pure number
      (bind _output_get_2 (set `/Game/TurnBasedJRPGTemplate/Blueprints/Units/BP_UnitBase.magicalDefense` 0 (`self.targetUnit`)))
      (return _output_get_2))))

(fn `Reduce Physical Defense`
  (params (isPercentage :type Boolean))
  (returns (newDefense :type Integer))
  (bind _targetunit (`self.targetUnit`))
  (bind _targetunit_2 (`self.targetUnit`))
  (if isPercentage
    ;[1 1 1] Reduce defense by percentage
    (set `/Game/TurnBasedJRPGTemplate/Blueprints/Units/BP_UnitBase.defense` (* (`/Game/TurnBasedJRPGTemplate/Blueprints/Units/BP_UnitBase.defense` _targetunit) (/ (- 100 (`self.defenseModifier`)) 100)) _targetunit)
    (else
      ;[1 1 1] Reduce defense by pure number
      (set `/Game/TurnBasedJRPGTemplate/Blueprints/Units/BP_UnitBase.defense` (- (`/Game/TurnBasedJRPGTemplate/Blueprints/Units/BP_UnitBase.defense` _targetunit_2) (`self.defenseModifier`)) _targetunit_2))))

(fn `UserConstructionScript`
  (`parent.UserConstructionScript`))