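; BP_CombatBuff_Stun is a combat buff that stuns its target unit for as long as it is active.
; On apply, it runs the parent logic, sets the unit's IsStun flag and plays that unit's stun montage.
; When the buff ends, it clears the flag and plays the idle montage.
; Initialization and construction only call the parent versions.
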(event `self.ApplyBuff`
  (bind _targetunit (`self.targetUnit`))
  (`parent.ApplyBuff`)
  (set `/Game/TurnBasedJRPGTemplate/Blueprints/Units/BP_UnitBase.isStun` true _targetunit)
  (`/Game/TurnBasedJRPGTemplate/Blueprints/Units/BP_UnitBase.PlayAnimationMontage` _targetunit (`/Game/TurnBasedJRPGTemplate/Blueprints/Units/BP_UnitBase.stunAnimationMontage` _targetunit)))

(event `self.OnBuffEnded`
  (bind _targetunit (`self.targetUnit`))
  (`parent.OnBuffEnded`)
  (set `/Game/TurnBasedJRPGTemplate/Blueprints/Units/BP_UnitBase.isStun` false _targetunit)
  (`/Game/TurnBasedJRPGTemplate/Blueprints/Units/BP_UnitBase.PlayAnimationMontage` _targetunit (`/Game/TurnBasedJRPGTemplate/Blueprints/Units/BP_UnitBase.IdleAnimationMontage` _targetunit)))

(fn `Initialization`
  (params (buffInitData :type "/Game/Combat/Blueprints/Skills/Buffs/BuffInitData Structure"))
  (`parent.Initialization` buffInitData))

(fn `UserConstructionScript`
  (`parent.UserConstructionScript`))