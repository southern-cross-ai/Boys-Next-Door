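; BP_Burn is a combat skill buff that visually marks the target unit as burning.
; On apply, it overrides LOD 0 vertex colors on the unit's skeletal mesh with a one-element array holding the target tint color and prints a debug message naming the unit.
; When the buff ends, it clears that override to restore the original colors.
; The graph itself contains no damage logic.
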(event `self.ApplyBuff`
  (bind _targetunit (`self.targetUnit`))
  (`SkinnedMeshComponent.SetVertexColorOverride_LinearColor` (`/Game/TurnBasedJRPGTemplate/Blueprints/Units/BP_UnitBase.SkeletalMesh` _targetunit) 0 (`|MakeArray` (`self.TargetTintColor`)))
  (`KismetSystemLibrary.PrintString` (`KismetStringLibrary.Concat_StrStr` "Burning Buff applied to unit " (`KismetSystemLibrary.GetObjectName` _targetunit))))

(event `self.OnBuffEnded`
  ;[1 1 1] 变回角色原有颜色
  (`SkinnedMeshComponent.ClearVertexColorOverride` (`/Game/TurnBasedJRPGTemplate/Blueprints/Units/BP_UnitBase.SkeletalMesh` (`self.targetUnit`)) 0))

(fn `UserConstructionScript`
  (`parent.UserConstructionScript`))