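; BP_CombatBuff_Terro is a combat buff that raises a player unit's pressure over time.
; Initialization takes the pressure amount from the buff init data's damage modifier field.
; Each turn effect runs the parent logic, casts the target to BP_CombatPlayerUnitBase, increases its pressure by that amount and prints a debug message.
; Other unit types only get an error print, while apply and end events just call the parent.
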(event `self.ApplyBuff`
  (`parent.ApplyBuff`))

(event `self.ProcessTurnEffect`
  (bind _pressuremodifier (`self.pressureModifier`))
  (`parent.ProcessTurnEffect`)
  ;[1 1 1] Increase pressure overtime
  (bind _asbp_combat_player_unit_base (cast `/Game/Combat/Blueprints/Unit/PlayerUnits/BP_CombatPlayerUnitBase` (`self.targetUnit`))
    (:`then`
      (`/Game/Combat/Blueprints/Unit/PlayerUnits/BP_CombatPlayerUnitBase.IncreasePressure` _asbp_combat_player_unit_base _pressuremodifier)
      ;[1 1 1] Debug print
      (`KismetSystemLibrary.PrintString` (`KismetStringLibrary.Concat_StrStr` "]'s pressure increased by " (`KismetStringLibrary.Conv_IntToString` _pressuremodifier))))
    (:`CastFailed`
      (`KismetSystemLibrary.PrintString` "Buff Terro can't be applied to a non-CombatPlayerUnitBase unit type or child type"))))

(event `self.OnBuffEnded`
  (`parent.OnBuffEnded`))

(fn `Initialization`
  (params (buffInitData :type "/Game/Combat/Blueprints/Skills/Buffs/BuffInitData Structure"))
  (`parent.Initialization` (struct))
  (set `self.pressureModifier` (`.modifierdamage_14_90B8CDA1433309480B2256B0A86C44E1` (break `/Game/Combat/Blueprints/Skills/Buffs/BuffInitData` buffInitData))))

(fn `UserConstructionScript`
  (`parent.UserConstructionScript`))