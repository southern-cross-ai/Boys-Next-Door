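; Combat skill Blueprint for Shield Bash, which damages the current target and knocks it back in the enemy line.
; The animation notify deals multiplier-scaled damage; on success, the enemy's position index drops by a random 1-2, clamped to 0-3.
; SwapPositionByIndex swaps it with any enemy occupying that slot, otherwise moves it to the empty spawn location and updates its index.
; The skill reports itself used when the animation ends.
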(event `/Game/TurnBasedJRPGTemplate/Blueprints/Skills/BP_SkillBase.UseSkill`
  (`self.PlaySkillAnimation`))

(event `self.UseSkillOnNotify`
  (bind _ishit (`/Game/TurnBasedJRPGTemplate/Blueprints/Battle/BP_BattleController.DealDamage` (`self.battleController`) 0 (`self.damageMultiplier`)))
  (if _ishit
    (bind _asbp_combat_enemy_unit_base (cast `/Game/Combat/Blueprints/Unit/EnemyUnits/BP_CombatEnemyUnitBase` (`/Game/TurnBasedJRPGTemplate/Blueprints/Battle/BP_BattleController.currentTargetUnit` (`self.battleController`))))
    ;[1 1 1] push the target 1-2 position behind
    (`/Engine/EditorBlueprintResources/StandardMacros.IsValid` _asbp_combat_enemy_unit_base
      (:`Is Valid`
        (bind _currentposition (`/Game/Combat/Blueprints/Unit/EnemyUnits/BP_CombatEnemyUnitBase.currentPosition` _asbp_combat_enemy_unit_base))
        (bind _output_get (set `self.indexToSwapWith` (`KismetMathLibrary.Clamp` (- _currentposition (`KismetMathLibrary.RandomIntegerInRange` 1 2)) 0 3)))
        (`self.SwapPositionByIndex` _currentposition _output_get)))))

(event `self.OnSkillAnimationEnded`
  (`/Game/TurnBasedJRPGTemplate/Blueprints/Skills/BP_SkillBase.OnSkillUsed`))

(fn `SwapPositionByIndex`
  (params (Source :type Integer) (SwapWith :type Integer))
  (bind _swapsourceenemy (`self.SwapSourceEnemy`))
  (bind _swaptargetenemy (`self.SwapTargetEnemy`))
  (if (not (== Source SwapWith))
    (set `self.SwapSourceEnemy` null)
    (set `self.SwapTargetEnemy` null)
    ;[1 1 1] Find Source and Target Enemy Unit
    (for _array_element (`/Game/TurnBasedJRPGTemplate/Blueprints/Battle/BP_BattleBase.enemyUnits` (`/Game/TurnBasedJRPGTemplate/Blueprints/Battle/BP_BattleController.currentBattle` (`self.battleController`)))
      (bind _asbp_combat_enemy_unit_base (cast `/Game/Combat/Blueprints/Unit/EnemyUnits/BP_CombatEnemyUnitBase` _array_element))
      (`/Engine/EditorBlueprintResources/StandardMacros.IsValid` _asbp_combat_enemy_unit_base
        (:`Is Valid`
          (bind _currentposition (`/Game/Combat/Blueprints/Unit/EnemyUnits/BP_CombatEnemyUnitBase.currentPosition` _asbp_combat_enemy_unit_base))
          (if (== _currentposition Source)
            (set `self.SwapSourceEnemy` _asbp_combat_enemy_unit_base)
            (elif (== _currentposition SwapWith)
              (set `self.SwapTargetEnemy` _asbp_combat_enemy_unit_base))))))
    (`/Engine/EditorBlueprintResources/StandardMacros.IsValid` _swaptargetenemy
      (:`Is Valid`
        (`/Game/Combat/Blueprints/Unit/EnemyUnits/BP_CombatEnemyUnitBase.Swap Position With` _swapsourceenemy _swaptargetenemy)
        (`KismetSystemLibrary.PrintString` (`KismetStringLibrary.Concat_StrStr` (`KismetStringLibrary.Concat_StrStr` (`KismetStringLibrary.Concat_StrStr` (`KismetStringLibrary.Concat_StrStr` "Enemy at position [" (`KismetStringLibrary.Conv_IntToString` (`/Game/Combat/Blueprints/Unit/EnemyUnits/BP_CombatEnemyUnitBase.currentPosition` _swapsourceenemy))) "]  Swap with enemy at [") (`KismetStringLibrary.Conv_IntToString` (`/Game/Combat/Blueprints/Unit/EnemyUnits/BP_CombatEnemyUnitBase.currentPosition` _swaptargetenemy))) "]")))
      (:`Is Not Valid`
        (`/Game/Combat/Blueprints/Unit/EnemyUnits/BP_CombatEnemyUnitBase.Move To Target With Root` _swapsourceenemy (`self.K2_GetActorLocation` (`|GetArrayItem` (`/Game/TurnBasedJRPGTemplate/Blueprints/Battle/BP_BattleBase.enemySpawnLocations` (`/Game/TurnBasedJRPGTemplate/Blueprints/Battle/BP_BattleController.currentBattle` (`self.battleController`))) SwapWith)) false 700.0)
        (set `/Game/Combat/Blueprints/Unit/EnemyUnits/BP_CombatEnemyUnitBase.currentPosition` SwapWith _swapsourceenemy)))))

(fn `UserConstructionScript`
  (`parent.UserConstructionScript`))