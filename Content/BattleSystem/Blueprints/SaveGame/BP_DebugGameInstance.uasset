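; Game instance Blueprint that provides an in-game debug window, a debug message log and console command execution.
; ToggleDebugWindow lazily creates the debug widget for the first player controller, then toggles its visibility on later calls.
; LogDebugMessage appends to DebugLogs, prints a confirmation and refreshes WBP_DebugWindow, with a function wrapper exposing the same event.
; ExecuteCommand passes a string to the console; its logging step is left unconnected.
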(event `ToggleDebugWindow`
  (bind _debugwidgetinstance (`self.DebugWidgetInstance`))
  ;[1 1 1] Instantiate the Debug Window if it does not exist, and toggle it's visibility.
  (if (and (not (`KismetSystemLibrary.IsValid` (`self.DebugWidgetInstance`))) (`KismetSystemLibrary.IsValidClass` (`self.DebugWidgetClass`)))
    (bind _returnvalue (`|CreateWidget` (`self.DebugWidgetClass`) (`GameplayStatics.GetPlayerController` 0)))
    (bind _output_get (set `self.DebugWidgetInstance` _returnvalue))
    (if (`KismetSystemLibrary.IsValid` _output_get)
      (`UserWidget.AddToViewport` _output_get 0)
      (`Widget.SetVisibility` _output_get "Visible"))
    (elif (`KismetSystemLibrary.IsValid` _debugwidgetinstance)
      (if (`Widget.IsVisible` _debugwidgetinstance)
        (`Widget.SetVisibility` _debugwidgetinstance "Hidden")
        (else
          (`Widget.SetVisibility` _debugwidgetinstance "Visible"))))))

(event `LogDebugMessage`
  (params (Message :type String))
  ;[1 1 1] Add the message into the debug logs array and update the debug window.
  (`KismetArrayLibrary.Array_Add` (`self.DebugLogs`) Message)
  (`KismetSystemLibrary.PrintString` (`KismetStringLibrary.Concat_StrStr` "Add " Message " to game instance debug logs"))
  (bind _aswbp_debug_window (cast `/Game/BattleSystem/Blueprints/Interfaces/WBP_DebugWindow` (`self.DebugWidgetInstance`)))
  (`/Game/BattleSystem/Blueprints/Interfaces/WBP_DebugWindow.UpdateDebugUI` _aswbp_debug_window))

(event `ExecuteCommand`
  (params (Command :type String))
  (`KismetSystemLibrary.ExecuteConsoleCommand` Command null))

(fn `F_LogDebugMessage`
  (params (Message :type String))
  (`self.LogDebugMessage` Message))