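; BP_BattleManager_Base is an early battle manager that starts a round-based battle on BeginPlay.
; Initialization fills HeroDatas with four placeholder heroes sharing fixed HP and random Speed, printing a separately rolled speed for each.
; The round loop's condition is false, so StartNewRound never runs; it only iterates the heroes with an empty body, leaving sorting and speed-variation nodes unconnected.
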(event `self.ReceiveBeginPlay`
  (`self.BattleStart`))

(event `BattleStart`
  (`self.BattleInitialization`)
  (while false
    (`self.StartNewRound`)))

(fn `BattleInitialization`
  (bind _returnvalue (`KismetMathLibrary.RandomInteger` 10))
  (`|ExecutionSequence`
    (:`then_0`
      (for _array_element (`|MakeArray` 0 1 2 3)
        (bind _returnvalue_2 (`KismetStringLibrary.Conv_IntToString` _array_element))
        (`KismetArrayLibrary.Array_Add` (`self.hero_datas`) (make `/Game/BattleSystem/Structures/S_HeroStatus_Main` _array_element _returnvalue_2 0 0 1 (make `/Game/BattleSystem/Structures/S_HeroStatus_Battle` 100 100 0 _returnvalue)))
        (`KismetSystemLibrary.PrintString` (`KismetStringLibrary.Concat_StrStr` (`KismetStringLibrary.Concat_StrStr` "Add new Hero: " _returnvalue_2) (`KismetStringLibrary.Concat_StrStr` "With Speed: " (`KismetStringLibrary.Conv_IntToString` _returnvalue))) true true (struct :`R` 1.0 :`B` 0.031066 :`A` 1.0))))
    (:`then_4`
      (return))))

(fn `StartNewRound`
  (`|ExecutionSequence`
    (:`then_0`
      (for _array_element (`self.hero_datas`)
        _))))

(fn `UserConstructionScript`)